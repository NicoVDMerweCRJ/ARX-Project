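; PictureFrame is an AR actor that draws a four-corner frame, apparently around a tracked image, tinted by image index and tracking state.
; BeginPlay creates one dynamic material instance and shares it across the four corner components.
; SetExtent moves the corners to half the given extent on X and Y.
; SetImage sets the Tint from a color array, lowering alpha when the state is not Tracking.
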(event EventBeginPlay
  (bind _returnvalue (Rendering|Material|CreateDynamicMaterialInstance "/Game/ARIR/Blueprints/Object/PictureFrameMaterial.PictureFrameMaterial" "None" :!class /Script/Engine.KismetMaterialLibrary))
  (bind _output_get (Variables|Default|SetPictureFrameDynamicMaterial _returnvalue))
  (Rendering|Material|SetMaterial (Variables|Default|GetUpperLeft) 0 _output_get)
  (Rendering|Material|SetMaterial (Variables|Default|GetUpperRight) 0 _output_get)
  (Rendering|Material|SetMaterial (Variables|Default|GetLowerLeft) 0 _output_get)
  (Rendering|Material|SetMaterial (Variables|Default|GetLowerRight) 0 _output_get))

(event Collision|EventActorBeginOverlap
  (params (OtherActor :type Actor%20Object%20Reference)))

(event EventTick
  (params (DeltaSeconds :type Float%20%28single-precision%29)))

(fn ConstructionScript)

(fn SetExtent
  (params (Extent :type Vector))
  (Transformation|SetRelativeLocation (Variables|Default|GetUpperLeft) (* Extent "0.500000,-0.500000,0.000000") false true)
  (Transformation|SetRelativeLocation (Variables|Default|GetUpperRight) (* Extent "0.500000,0.500000,0.000000") false true)
  (Transformation|SetRelativeLocation (Variables|Default|GetLowerRight) (* Extent "-0.500000,0.500000, 0") false true)
  (Transformation|SetRelativeLocation (Variables|Default|GetLowerLeft) (* Extent "-0.500000,-0.500000, 0") false true))

(fn SetImage
  (params (ImageIndex :type Integer) (TrackingState :type EARTrackingState%20Enum :default "Unknown"))
  (bind _colorselection (Variables|Default|GetColorSelection))
  (bind _output (Utilities|Array|Get(acopy) _colorselection ImageIndex))
  (bind (_b _g _r) (Math|Color|BreakColor _output))
  (Rendering|Material|SetVectorParameterValue (Variables|Default|GetPictureFrameDynamicMaterial) "Tint" (Math|Conversions|ToLinearColor(Color) (Math|Color|MakeColor _b _g _r (select (Utilities|Enum|Equal(Enum) TrackingState "Tracking") 255 64))) :!class /Script/Engine.MaterialInstanceDynamic))